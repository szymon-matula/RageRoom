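; Destructible ceramic sink for the rage room level that breaks when struck by a weapon.
; Either of two trigger boxes reacts to an overlapping actor tagged "Weapon" while the sink is not yet destroyed.
; A hit spawns an FS_MasterField actor at the sink's transform through AddForce, plays the ceramic breaking sound and sets IsDestroyed so it fires only once.
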(event `Add Force`
  (params (SpawnTransform :type "Transform Structure"))
  (`|SpawnActorFromClass` "/Engine/EditorResources/FieldNodes/FS_MasterField.FS_MasterField_C" SpawnTransform "Undefined" "MultiplyWithRoot" null null))

(event `self.Box.OnComponentBeginOverlap`
  (params (OverlappedComponent :type "PrimitiveComponent Object Reference") (OtherActor :type "Actor Object Reference") (OtherComp :type "PrimitiveComponent Object Reference") (OtherBodyIndex :type Integer) (bFromSweep :type Boolean) (SweepResult :type "HitResult Structure (by ref)"))
  (if (`self.IsDestroyed`)
    _
    (elif (`self.ActorHasTag` OtherActor "Weapon")
      (`/Engine/EditorBlueprintResources/StandardMacros.DoOnce` false
        (:`Completed`
          (`self.Add Force` (`self.GetTransform`))
          (`GameplayStatics.PlaySoundAtLocation` "/Game/RageRoomLevel/Sounds/Ceramic/sink-ceramic-breaking.sink-ceramic-breaking" (`self.K2_GetActorLocation`) (struct) 1.0 1.0 0.0 null null null null)
          (set `self.IsDestroyed` true))))))

(event `self.Box1.OnComponentBeginOverlap`
  (params (OverlappedComponent :type "PrimitiveComponent Object Reference") (OtherActor :type "Actor Object Reference") (OtherComp :type "PrimitiveComponent Object Reference") (OtherBodyIndex :type Integer) (bFromSweep :type Boolean) (SweepResult :type "HitResult Structure (by ref)"))
  (if (`self.IsDestroyed`)
    _
    (elif (`self.ActorHasTag` OtherActor "Weapon")
      (`/Engine/EditorBlueprintResources/StandardMacros.DoOnce` false
        (:`Completed`
          (`self.Add Force` (`self.GetTransform`))
          (`GameplayStatics.PlaySoundAtLocation` "/Game/RageRoomLevel/Sounds/Ceramic/sink-ceramic-breaking.sink-ceramic-breaking" (`self.K2_GetActorLocation`) (struct) 1.0 1.0 0.0 null null null null)
          (set `self.IsDestroyed` true))))))

(fn `UserConstructionScript`)